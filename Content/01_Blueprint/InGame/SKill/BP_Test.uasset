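; BP_Test is a test skill actor that follows its owner's location while spinning a sphere component and its children around it.
; BeginPlay unhides the sphere's child components by index.
; Tick adds a small rotation to the sphere each frame and snaps the actor to the owner's position.
; The SetOn function is an empty stub, and an even angular-spacing calculation is left unconnected.
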(event `self.ReceiveBeginPlay`
  (for _index (range (`self.Num`))
    (`SceneComponent.SetHiddenInGame` (`SceneComponent.GetChildComponent` (`self.Sphere`) _index) false false)))

(event `self.ReceiveTick`
  (params (DeltaSeconds :type "Float (single-precision)"))
  (`SceneComponent.K2_AddRelativeRotation` (`self.Sphere`) (struct :`Yaw` 1.0) false false)
  (`self.K2_SetActorLocation` (`self.K2_GetActorLocation` (`self.GetOwner`))))

(fn `set On`
  (params (`타깃` :type "SceneComponent Object Reference")))

(fn `UserConstructionScript`)